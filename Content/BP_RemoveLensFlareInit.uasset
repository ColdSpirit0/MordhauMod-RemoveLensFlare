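; Actor blueprint that removes lens flare from the level's post process volumes, running only where cosmetic events can execute.
; On BeginPlay it polls every half second until the GameState is valid, then waits another half second before calling RemoveLensFlare.
; That event finds every PostProcessVolume and sets an intensity member of its settings to zero.
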(event `self.ReceiveBeginPlay`
  (`/Engine/EditorBlueprintResources/StandardMacros.Can Execute Cosmetic Events`
    (:`True`
      ;[1 1 1] Wait for map initialized
      (`/Engine/EditorBlueprintResources/StandardMacros.IsValid` (`GameplayStatics.GetGameState`) :!label _label
        (:`Is Valid`
          (`KismetSystemLibrary.Delay` 0.5)
          (`self.RemoveLensFlare`))
        (:`Is Not Valid`
          (`KismetSystemLibrary.Delay` 0.5)
          (goto _label))))))

(event `RemoveLensFlare`
  (`/Engine/EditorBlueprintResources/StandardMacros.Can Execute Cosmetic Events`
    (:`True`
      (bind _outactors (`GameplayStatics.GetAllActorsOfClass` "/Script/Engine.PostProcessVolume"))
      (for _array_element _outactors
        (setmembers `PostProcessSettings` :`StructRef` (`PostProcessVolume.Settings` _array_element) :`LensFlareIntensity` 0.0)))))

(fn `UserConstructionScript`
  (`parent.UserConstructionScript`))